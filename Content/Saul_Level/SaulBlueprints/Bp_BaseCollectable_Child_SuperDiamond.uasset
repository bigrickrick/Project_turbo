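; Super diamond collectable, a child of the base collectable that awards its collectable value as points when collected.
; Its Collect event plays a charge sound at world origin, then an announcer clip and Niagara explosion at the actor's location.
; It adds the value directly to the coin widget's Points through the third-person game mode, with debug prints.
; The event neither calls the parent version nor destroys the actor.
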(event EventBeginPlay
  (|CallParentFunction) ; This node is disabled and will not be called.\nDrag off pins to build functionality.
)

(event Collision|EventActorBeginOverlap
  (params (OtherActor :type Actor%20Object%20Reference)))

(event EventTick
  (params (DeltaSeconds :type Float%20%28single-precision%29)))

(event EventCollect
  (params (Collector :type Actor%20Object%20Reference))
  (Audio|PlaySoundatLocation "/Game/RawContent/CollectableSounds/MEGAMAN_X_BUSTER_CHARGE_SOUND.MEGAMAN_X_BUSTER_CHARGE_SOUND" "0, 0, 0" "0, 0, 0" 1.0 1.0 0.0 0 0 0 0)
  (Niagara|SpawnSystematLocation "/Game/Saul_Level/NS_Explosion.NS_Explosion" (Transformation|GetActorLocation))
  (Development|PrintString "collect +1000")
  (Audio|PlaySoundatLocation "/Game/RawContent/CollectableSounds/Crazy_Taxi__1999__In_Game_Announcer-VEED.Crazy_Taxi__1999__In_Game_Announcer-VEED" (Transformation|GetActorLocation) "0, 0, 0" 7.0 1.0 0.5 0 0 0 0)
  (bind _asbp_third_person_game_mode (Utilities|Casting|CastToBP_ThirdPersonGameMode (Game|GetGameMode)))
  (Variables|Default|SetisCollecting true)
  (bind _output_get (Variables|/Game/Saul_Level/CoinWidget.CoinWidget_C|SetPoints (Variables|/Game/ThirdPerson/Blueprints/BP_ThirdPersonGameMode.BP_ThirdPersonGameMode_C|GetCoinWidgetReference _asbp_third_person_game_mode) (+ (Variables|Default|GetBaseCollectableValue) (Variables|/Game/Saul_Level/CoinWidget.CoinWidget_C|GetPoints (Variables|/Game/ThirdPerson/Blueprints/BP_ThirdPersonGameMode.BP_ThirdPersonGameMode_C|GetCoinWidgetReference _asbp_third_person_game_mode)))))
  (Variables|Default|SetisCollecting false)
  (Development|PrintText (Utilities|Text|ToText(Integer) _output_get)))

(fn ConstructionScript
  (|CallParentFunction))