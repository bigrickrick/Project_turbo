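; Base small collectable pickup that hops in place and is collected when the player touches it.
; Shortly after BeginPlay, a looping timer with slight start variance applies an upward impulse to the mesh for each hop.
; Overlap of the sphere by a Player-tagged actor calls Collect, which plays a sound at world origin, spawns Niagara particles and prints a debug message, then the actor is destroyed.
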(event OnComponentBeginOverlap(Sphere)
  (params (OverlappedComponent :type Primitive%20Component%20Object%20Reference) (OtherActor :type Actor%20Object%20Reference) (OtherComp :type Primitive%20Component%20Object%20Reference) (OtherBodyIndex :type Integer) (bFromSweep :type Boolean) (SweepResult :type Hit%20Result%20Structure%20%28by%20ref%29))
  (if (Actor|ActorHasTag OtherActor "Player")
    (CallFunction|Collect)
    (Actor|DestroyActor)))

(event Custom|Hop
  (Physics|AddImpulse (Variables|Debug|GetStaticMeshComponent) "0.000000,0.000000,16327.000000" "None" false))

(event Custom|Collect
  (params (Collector :type Actor%20Object%20Reference))
  (Audio|PlaySoundatLocation "/Game/RawContent/CollectableSounds/Collectable_Sound_New_Skill_.Collectable_Sound_New_Skill_" "0, 0, 0" "0, 0, 0" 1.0 1.0 0.0 0 0 0 0)
  (Niagara|SpawnSystematLocation "/Game/Saul_Level/Ns_ParticleSystemCollectable10.Ns_ParticleSystemCollectable10" (Transformation|GetActorLocation))
  (Development|PrintString "Collect+1"))

(event EventBeginPlay
  (Utilities|FlowControl|Delay 0.2)
  (Utilities|Time|SetTimerbyEvent (delegate Custom|Hop) 1.0 true false 0.0 0.3))

(fn ConstructionScript)