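; BP_SuperDeathWallRed is a resizable hazard that sends the player character back to the last checkpoint on contact.
; When the Floor component is hit by a Prototype_Character, it teleports that character to the Box location of LastCheckpoint stored on BP_ThirdPersonGameMode, with zero rotation.
; The construction script scales Floor in X and Y from the Size variable divided by 100, keeping Z at unit scale.
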(event OnComponentHit(Floor)
  (params (HitComponent :type Primitive%20Component%20Object%20Reference) (OtherActor :type Actor%20Object%20Reference) (OtherComp :type Primitive%20Component%20Object%20Reference) (NormalImpulse :type Vector :default "0, 0, 0") (Hit :type Hit%20Result%20Structure%20%28by%20ref%29))
  (bind _asprototype_character (Utilities|Casting|CastToPrototype_Character OtherActor))
  (bind _asbp_third_person_game_mode (Utilities|Casting|CastToBP_ThirdPersonGameMode (Game|GetGameMode)))
  (Transformation|Teleport _asprototype_character (Transformation|GetWorldLocation (Variables|/Game/MaxStuff/Blueprints/BP_Checkpoint.BP_Checkpoint_C|GetBox (Variables|/Game/ThirdPerson/Blueprints/BP_ThirdPersonGameMode.BP_ThirdPersonGameMode_C|GetlastCheckpoint _asbp_third_person_game_mode))) "0, 0, 0"))

(fn ConstructionScript
  (Utilities|FlowControl|Sequence
    (:then_0
      (Transformation|SetRelativeScale3D (Variables|Default|GetFloor) (CallFunction|GetNormalSize)))))

(fn GetNormalSize
  (bind _size (Variables|Settings|GetSize))
  (bind _returnvalue (/ _size 1e+02))
  (return (Math|Vector|MakeVector (.x _returnvalue) (.y _returnvalue) 1.0)))